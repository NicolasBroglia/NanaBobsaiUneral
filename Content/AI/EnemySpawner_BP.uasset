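; Enemy spawner actor that creates waves of melee enemies at its own transform, growing larger with each wave.
; On BeginPlay it casts the game mode to ThirdPersonGameMode and binds SpawnEnemy to its RespawnEnemy dispatcher.
; Each call spawns the current count of Enemy_Melee actors, then raises an increment and adds it to that count, so the step between waves keeps widening.
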(event `self.ReceiveBeginPlay`
  (bind _asthird_person_game_mode (cast `/Game/ThirdPersonBP/Blueprints/ThirdPersonGameMode` (`GameplayStatics.GetGameMode`)))
  (add `/Game/ThirdPersonBP/Blueprints/ThirdPersonGameMode.RespawnEnemy` _asthird_person_game_mode (delegate `SpawnEnemy`)))

(event `SpawnEnemy`
  (for _ (range (`self.EnemySpawned`))
    (`|SpawnActorFromClass` "/Game/AI/Enemy_Melee.Enemy_Melee_C" (`self.GetTransform`) "Undefined" "OverrideRootScale" null null))
  (`/Engine/EditorBlueprintResources/StandardMacros.IncrementInt` (`self.EnemyIncrement`)
    (:`  `
      (set `self.EnemySpawned` (+ (`self.EnemySpawned`) (`self.EnemyIncrement`))))))

(fn `UserConstructionScript`)