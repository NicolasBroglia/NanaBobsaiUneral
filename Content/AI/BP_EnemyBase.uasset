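; Base enemy character that chases a target player, makes melee attacks and tracks its own health.
; ChasePlayer uses AIMoveTo, then Attack plays a montage whose notify applies damage through a sphere overlap.
; A hit resumes the chase after a delay; a miss does not.
; Death decrements the game mode's alive count, triggers its remaining-enemy check and destroys the actor; death animation and count increment are unwired.
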(event `self.ReceiveAnyDamage`
  (params (Damage :type "Float (single-precision)") (DamageType :type "DamageType Object Reference") (InstigatedBy :type "Controller Object Reference") (DamageCauser :type "Actor Object Reference"))
  ;[1 1 1] Health
  (if (not (`self.IsDead`))
    (set `self.Health` (- (`self.Health`) Damage))
    (if (<= (`self.Health`) 0.0)
      (`self.Death`))))

(event `self.ReceiveBeginPlay`)

(event `ChasePlayer`
  (params (Target :type "Pawn Object Reference"))
  (set `self.playerTarget` Target)
  (if (not (`self.IsDead`))
    (`|AIMoveTo` self (0.0 0.0 0.0) Target
      (:`OnSuccess`
        (`self.Attack`)))))

(event `Death`
  (set `self.IsDead` true)
  (bind _asthird_person_game_mode (cast `/Game/ThirdPersonBP/Blueprints/ThirdPersonGameMode` (`GameplayStatics.GetGameMode`)))
  (`/Engine/EditorBlueprintResources/StandardMacros.DecrementInt` (`/Game/ThirdPersonBP/Blueprints/ThirdPersonGameMode.EnemyAlive` _asthird_person_game_mode)
    (:`  `
      (`/Game/ThirdPersonBP/Blueprints/ThirdPersonGameMode.CheckEnemyLeft` _asthird_person_game_mode)
      (`self.K2_DestroyActor`))))

(event `Attack`
  ;[1 1 1] AttackLogic
  (`|PlayMontage` (`self.Mesh`) (`self.AtkA`)
    (:`OnNotifyBegin`
      (bind _outactors (`KismetSystemLibrary.SphereOverlapActors` (`SceneComponent.K2_GetComponentLocation` (`self.CollisionSphere`)) 100.0 (`|MakeArray` "ObjectTypeQuery3" :!type "EObjectTypeQuery Enum") "/Game/ThirdPersonBP/Blueprints/ThirdPersonCharacter.ThirdPersonCharacter_C"))
      (for _array_element _outactors
        (`GameplayStatics.ApplyDamage` _array_element (`self.Base Damage`) null self "/Script/Engine.DamageType")
        (`KismetSystemLibrary.Delay` 1.0)
        (`self.ChasePlayer` (`self.playerTarget`))))))

(fn `UserConstructionScript`)